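; BP_HUDChallengeGameInstance is a game instance that holds ammo, reload, booster and HUD state for a HUD challenge game.
; Init fills ammo to maximum, and HandleReload sets a reloading flag, waits for the reload time, then refills unless ammo is already full.
; ObtainBoost and ObtainHud set their unlock flags and notify the first-person character, BP_FPC, through a cast of the player character.
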(event Custom|ObtainBoost
  (Variables|Default|SetbBoosterEnabled true)
  (bind _asbp_fpc (Utilities|Casting|CastToBP_FPC (Game|GetPlayerCharacter 0)))
  (Default|ObtainBooster _asbp_fpc))

(event Custom|ObtainHud
  (Variables|Default|SetbHasHud true)
  (bind _asbp_fpc (Utilities|Casting|CastToBP_FPC (Game|GetPlayerCharacter 0)))
  (Default|ObtainHUD _asbp_fpc))

(event Custom|HandleReload
  (if (not (== (Variables|Default|GetCurrentAmmo) (Variables|Default|GetMaxAmmo)))
    (Variables|Default|SetbIsReloading true)
    (Utilities|FlowControl|Delay (Variables|Default|GetReloadTime))
    (Variables|Default|SetbIsReloading false)
    (Variables|Default|SetCurrentAmmo (Variables|Default|GetMaxAmmo))))

(event EventInit
  (Variables|Default|SetCurrentAmmo (Variables|Default|GetMaxAmmo)))