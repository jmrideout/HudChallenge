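; BP_MeteorSpawner is an actor that spawns enlarged BP_Meteor actors at random points inside its box, using the spawner's rotation.
; StartSpawning re-arms a timer that calls itself, then re-rolls the wait between MinWait and MaxWait, so each new delay applies to the following timer.
; StopSpawning clears that timer.
; BeginPlay is empty, so spawning begins only when StartSpawning is called.
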(event Custom|StartSpawning
  (Utilities|IsValid 0
    (:Is%20Valid
      (Utilities|Time|ClearandInvalidateTimerbyHandle (Variables|Default|GetSpawnTimer)))
    (:Is%20Not%20Valid
      _))
  (bind _returnvalue (Utilities|Time|SetTimerbyFunctionName 0 "StartSpawning" (Variables|Default|GetRandomWait)))
  (Variables|Default|SetSpawnTimer _returnvalue)
  (Variables|Default|SetRandomWait (Math|Random|RandomFloatinRange (Variables|Default|GetMinWait) (Variables|Default|GetMaxWait)))
  (Game|SpawnActorfromClass "/Game/MyContent/Blueprints/BP_Meteor.BP_Meteor_C" (Math|Transform|MakeTransform (Math|Random|RandomPointinBoundingBox (Transformation|GetActorLocation) (Variables|/Script/Engine.BoxComponent|GetBoxExtent (Variables|Default|GetBox))) (Transformation|GetActorRotation) "2.000000,2.000000,2.000000") "Undefined" 0 0))

(event Custom|StopSpawning
  (Utilities|Time|ClearandInvalidateTimerbyHandle (Variables|Default|GetSpawnTimer)))

(event EventBeginPlay)

(fn ConstructionScript)