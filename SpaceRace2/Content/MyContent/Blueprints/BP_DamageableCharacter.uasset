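; BP_DamageableCharacter is a damageable actor that shows the amount of damage it takes as text in the world.
; On AnyDamage, if the first player character is valid, it spawns a BP_DamageText at its own location, raised by a configurable height offset.
; The text is rotated to face that player at spawn and set to the damage value; no health is tracked here.
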(event Game|Damage|EventAnyDamage
  (params (Damage :type Float%20%28single-precision%29) (DamageType :type Damage%20Type%20Object%20Reference) (InstigatedBy :type Controller%20Object%20Reference) (DamageCauser :type Actor%20Object%20Reference))
  (Utilities|IsValid (Game|GetPlayerCharacter 0)
    (:Is%20Valid
      (bind _returnvalue (Game|SpawnActorfromClass "/Game/MyContent/Blueprints/BP_DamageText.BP_DamageText_C" (Math|Transform|MakeTransform (+ (Transformation|GetActorLocation) (Math|Vector|MakeVector 0.0 0.0 (Variables|Default|GetDamageTextCharacterHeightOffset))) (Math|Rotator|FindLookatRotation (Transformation|GetActorLocation) (Transformation|GetActorLocation (Game|GetPlayerCharacter 0)))) "AlwaysSpawn" 0 0))
      (Default|SetText _returnvalue (Utilities|Text|ToText(Float) Damage "HalfToEven" false true 1 324 0 1)))))

(fn ConstructionScript)