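; BP_3DRadarColor is a 3D radar display that shows the player character's detected actors as blips around its own location.
; Each tick it destroys the previous blips and spawns a BP_3DBlip for every entry in BP_FPC's DetectedActors.
; Blip positions are world-space offsets from the character multiplied by RadarScale, without rotation.
; MiddleAxis takes the first-person camera's world rotation as its relative rotation to show view direction.
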(event Custom|UpdateBlips
  (Utilities|IsValid (Variables|Default|GetChar)
    (:Is%20Valid
      (for _array_element (Variables|/Game/MyContent/Blueprints/BP_FPC.BP_FPC_C|GetDetectedActors (Variables|Default|GetChar))
        (Utilities|IsValid _array_element
          (:Is%20Valid
            (bind _returnvalue (Game|SpawnActorfromClass "/Game/MyContent/Blueprints/BP_3DBlip.BP_3DBlip_C" (Math|Transform|MakeTransform (+ (Transformation|GetActorLocation) (* (- (Transformation|GetActorLocation _array_element) (Transformation|GetActorLocation (Variables|Default|GetChar))) (Variables|Default|GetRadarScale)))) "Undefined" 0 0))
            (Utilities|Array|AddUnique (Variables|Default|GetBlips) _returnvalue)))))))

(event EventTick
  (params (DeltaSeconds :type Float%20%28single-precision%29))
  (Utilities|IsValid (Variables|Default|GetChar)
    (:Is%20Valid
      (for _array_element (Variables|Default|GetBlips)
        (Utilities|IsValid _array_element
          (:Is%20Valid
            (Actor|DestroyActor _array_element))))
      (Utilities|Array|Clear (Variables|Default|GetBlips))
      (Utilities|FlowControl|Sequence
        (:then_0
          (CallFunction|UpdateBlips))
        (:then_1
          (Transformation|SetRelativeLocationAndRotation (Variables|Default|GetMiddleAxis) "0, 0, 0" (Transformation|GetWorldRotation (Variables|/Game/MyContent/Blueprints/BP_FPC.BP_FPC_C|GetFirstPersonCamera (Variables|Default|GetChar))) false false))))))

(event EventBeginPlay
  (bind _returnvalue (Game|GetPlayerCharacter 0))
  (Utilities|IsValid _returnvalue
    (:Is%20Valid
      (bind _asbp_fpc (Utilities|Casting|CastToBP_FPC _returnvalue))
      (Variables|Default|SetChar _asbp_fpc))))

(fn ConstructionScript)