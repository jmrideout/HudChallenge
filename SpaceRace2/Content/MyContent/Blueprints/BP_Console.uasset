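; BP_Console is an interactable console that loads the Planet level when the player presses Use within its trigger box.
; A capsule component entering the box enables input on the console and spawns a BP_ConsoleUI actor at a rotation-relative offset above it.
; A DoOnce guards against duplicate UI spawns; leaving the box disables input, and if the UI is valid, destroys it and resets the guard.
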(event OnComponentBeginOverlap(Box)
  (params (OverlappedComponent :type Primitive%20Component%20Object%20Reference) (OtherActor :type Actor%20Object%20Reference) (OtherComp :type Primitive%20Component%20Object%20Reference) (OtherBodyIndex :type Integer) (bFromSweep :type Boolean) (SweepResult :type Hit%20Result%20Structure%20%28by%20ref%29))
  (bind _returnvalue (Transformation|GetActorRotation))
  (Utilities|Casting|CastToCapsuleComponent OtherComp)
  (Input|EnableInput (Game|GetPlayerController 0))
  (Utilities|FlowControl|DoOnce false
    (:Completed
      (bind _returnvalue_2 (Game|SpawnActorfromClass "/Game/MyContent/Blueprints/BP_ConsoleUI.BP_ConsoleUI_C" (Math|Transform|MakeTransform (+ (Math|Vector|RotateVector (Math|Vector|MakeVector 0.0 -2e+01 1.4e+02) _returnvalue) (Transformation|GetActorLocation)) _returnvalue (Transformation|GetActorScale3D)) "Undefined" 0 0))
      (Variables|Default|SetUI _returnvalue_2))))

(event OnComponentEndOverlap(Box)
  (params (OverlappedComponent :type Primitive%20Component%20Object%20Reference) (OtherActor :type Actor%20Object%20Reference) (OtherComp :type Primitive%20Component%20Object%20Reference) (OtherBodyIndex :type Integer))
  (bind _returnvalue (Transformation|GetActorRotation))
  (Utilities|Casting|CastToCapsuleComponent OtherComp)
  (Input|DisableInput (Game|GetPlayerController 0))
  (Utilities|IsValid (Variables|Default|GetUI)
    (:Is%20Valid
      (Actor|DestroyActor (Variables|Default|GetUI))
      (Utilities|FlowControl|DoOnce false) ; enters at Reset
    )))

(event Input|ActionEvents|InputActionUse
  (params (Key :type Key%20Structure :default "None"))
  (:Pressed
    (Game|OpenLevel(byName) "Planet")))

(fn ConstructionScript)