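; BP_Meteor is a meteor actor that explodes on impact and shows its speed on an attached tracker widget.
; On BeginPlay it turns to a random direction within a narrow cone around its forward vector.
; Each tick it turns the widget's axis toward the player character and writes raw velocity magnitude, labeled MPH without conversion, into W_Tracker.
; On hit it spawns an explosion effect and sound, then destroys itself.
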(event EventBeginPlay
  (Transformation|SetActorRotation (Math|Rotator|MakeRotfromXZ (Math|Random|RandomUnitVectorinConeinDegrees (Transformation|GetActorForwardVector) 15.0) (Transformation|GetActorUpVector))))

(event Collision|EventHit
  (params (MyComp :type Primitive%20Component%20Object%20Reference) (Other :type Actor%20Object%20Reference) (OtherComp :type Primitive%20Component%20Object%20Reference) (bSelfMoved :type Boolean) (HitLocation :type Vector :default "0, 0, 0") (HitNormal :type Vector :default "0, 0, 0") (NormalImpulse :type Vector :default "0, 0, 0") (Hit :type Hit%20Result%20Structure%20%28by%20ref%29))
  (bind _returnvalue (Transformation|GetActorLocation))
  ;[1 1 1] Spawn explosion at hit location and disappear
  (Effects|SpawnEmitteratLocation "/Game/MyContent/Misc/P_MeteorExplosion.P_MeteorExplosion" _returnvalue "0, 0, 0" "10.000000,10.000000,10.000000")
  (Audio|PlaySoundatLocation "/Game/MyContent/Misc/MeteorExplosion.MeteorExplosion" _returnvalue "0, 0, 0" 2.0 1.0 0.0 0 0 0)
  (Actor|DestroyActor))

(event EventTick
  (params (DeltaSeconds :type Float%20%28single-precision%29))
  ;[1 1 1] Rotate widget to face camera
  (Transformation|SetWorldRotation (Variables|Default|GetRotationAxis) (Math|Rotator|FindLookatRotation (Transformation|GetActorLocation) (Transformation|GetActorLocation (Game|GetPlayerCharacter 0))) false false)
  (bind _asw_tracker (Utilities|Casting|CastToW_Tracker (UserInterface|GetUserWidgetObject (Variables|Default|GetWidget))))
  (Default|InitializeTracker _asw_tracker (Utilities|Text|ToText(String) (Utilities|String|Append (Utilities|String|ToString(Float) (Math|Vector|VectorLength (Transformation|GetVelocity))) " MPH"))))

(fn ConstructionScript)