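; BP_MeteorStatic is a meteor actor with a tracker widget that faces the player and displays the meteor's speed.
; On BeginPlay it initializes the W_Tracker widget with the Info from its ACTrackerStats component.
; Each tick it turns RotationAxis toward the player character and reinitializes the tracker with its raw velocity magnitude labeled MPH, without unit conversion, replacing the initial text.
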(event EventBeginPlay
  (bind _asw_tracker (Utilities|Casting|CastToW_Tracker (UserInterface|GetUserWidgetObject (Variables|Default|GetWidget))))
  (Default|InitializeTracker _asw_tracker (Variables|/Game/MyContent/Blueprints/AC_TrackerStats.AC_TrackerStats_C|GetInfo (Variables|Default|GetAC_TrackerStats))))

(event EventTick
  (params (DeltaSeconds :type Float%20%28single-precision%29))
  (bind _returnvalue (Game|GetPlayerCharacter 0))
  ;[1 1 1] Rotate widget to face camera
  (Utilities|IsValid _returnvalue
    (:Is%20Valid
      (Transformation|SetWorldRotation (Variables|Default|GetRotationAxis) (Math|Rotator|FindLookatRotation (Transformation|GetActorLocation) (Transformation|GetActorLocation _returnvalue)) false false)
      (bind _asw_tracker (Utilities|Casting|CastToW_Tracker (UserInterface|GetUserWidgetObject (Variables|Default|GetWidget))))
      (Default|InitializeTracker _asw_tracker (Utilities|Text|ToText(String) (Utilities|String|Append (Utilities|String|ToString(Float) (Math|Vector|VectorLength (Transformation|GetVelocity))) " MPH"))))))

(fn ConstructionScript)