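; BP_DamageText is a floating damage number actor that displays a supplied text through a TextRender component.
; On BeginPlay it runs a timeline that lerps the actor upward from its spawn location by RiseAmount while fading the red text's alpha to zero.
; The actor destroys itself when the timeline finishes, and a SetText event lets the spawner set the displayed damage value.
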(event Custom|SetText
  (params (DamageNumberText :type Text))
  (Rendering|Components|TextRender|SetText (Variables|Default|GetTextRender) DamageNumberText))

(event EventBeginPlay
  (Variables|Default|SetInitialLocation (Transformation|GetActorLocation))
  (bind (_direction _positionalpha _fadealpha) (Timeline|PostionFadeDriver PlayFromStart)
    (:Update
      (Transformation|SetActorLocation (Math|Vector|Lerp(Vector) (Variables|Default|GetInitialLocation) (Math|Vector|MakeVector (.X (Math|Vector|BreakVector (Variables|Default|GetInitialLocation))) (.Y (Math|Vector|BreakVector (Variables|Default|GetInitialLocation))) (+ (.Z (Math|Vector|BreakVector (Variables|Default|GetInitialLocation))) (Variables|Default|GetRiseAmount))) _positionalpha) false false)
      (Rendering|Components|TextRender|SetTextRenderColor (Variables|Default|GetTextRender) (Math|Color|MakeColor 20 20 255 (Math|Conversions|ToByte(Integer) (Math|Float|Truncate (Math|Float|Lerp 255.0 0.0 _fadealpha))))))
    (:Finished
      (Actor|DestroyActor))))

(fn ConstructionScript)