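; BP_BoosterUpgrade is a pickup actor that grants the player a boost.
; When a capsule component overlaps its StaticMesh, a DoOnce gate lets it call ObtainBoost on BP_HUDChallengeGameInstance.
; It then plays a pickup sound at its location behind a validity check, plus a 2D beep, and destroys itself.
; The overlap filters only on component type, with no check on the owning actor.
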(event OnComponentBeginOverlap(StaticMesh)
  (params (OverlappedComponent :type Primitive%20Component%20Object%20Reference) (OtherActor :type Actor%20Object%20Reference) (OtherComp :type Primitive%20Component%20Object%20Reference) (OtherBodyIndex :type Integer) (bFromSweep :type Boolean) (SweepResult :type Hit%20Result%20Structure%20%28by%20ref%29))
  (Utilities|Casting|CastToCapsuleComponent OtherComp)
  (Utilities|FlowControl|DoOnce false
    (:Completed
      (bind _asbp_hudchallenge_game_instance (Utilities|Casting|CastToBP_HUDChallengeGameInstance (Game|GetGameInstance)))
      (Default|ObtainBoost _asbp_hudchallenge_game_instance)
      (Utilities|IsValid 0
        (:Is%20Valid
          (Audio|PlaySoundatLocation (Variables|Default|GetBoostPickupSound) (Transformation|GetActorLocation) "0, 0, 0" 1.0 1.0 0.0 0 0 0))
        (:Is%20Not%20Valid
          _))
      (Audio|PlaySound2D "/Game/MyContent/Misc/263133__pan14__tone-beep_Cue.263133__pan14__tone-beep_Cue" 1.0 1.0 0.0 0 0)
      (Actor|DestroyActor))))

(event EventBeginPlay)

(event Collision|EventActorBeginOverlap
  (params (OtherActor :type Actor%20Object%20Reference)))

(event EventTick
  (params (DeltaSeconds :type Float%20%28single-precision%29)))

(fn ConstructionScript)