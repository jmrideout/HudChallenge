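; BP_DamageArea is a box volume that deals caustic damage to a BP_FPC character inside it.
; When the character's capsule enters, it applies instant damage and starts a looping timer that damages the single stored character each tick.
; Any capsule leaving the box clears that timer.
; The construction script sizes the box from the X, Y and Z variables.
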(event OnComponentBeginOverlap(Box)
  (params (OverlappedComponent :type Primitive%20Component%20Object%20Reference) (OtherActor :type Actor%20Object%20Reference) (OtherComp :type Primitive%20Component%20Object%20Reference) (OtherBodyIndex :type Integer) (bFromSweep :type Boolean) (SweepResult :type Hit%20Result%20Structure%20%28by%20ref%29))
  ;[1 1 1] Apply instant and periodic damage while inside
  (bind _ascapsule_collision (Utilities|Casting|CastToCapsuleComponent OtherComp))
  (bind _asbp_fpc (Utilities|Casting|CastToBP_FPC (Components|GetOwner _ascapsule_collision)))
  (Variables|Default|SetChar _asbp_fpc)
  (Game|Damage|ApplyDamage _asbp_fpc (Variables|Default|GetInstantDamage) 0 self "/Game/MyContent/Blueprints/BP_CausticDamageType.BP_CausticDamageType_C")
  (bind _returnvalue (Utilities|Time|SetTimerbyEvent (delegate Custom|DamageTick) (Variables|Default|GetDamageTickDelay) true))
  (Variables|Default|SetDamageTickTimer _returnvalue))

(event OnComponentEndOverlap(Box)
  (params (OverlappedComponent :type Primitive%20Component%20Object%20Reference) (OtherActor :type Actor%20Object%20Reference) (OtherComp :type Primitive%20Component%20Object%20Reference) (OtherBodyIndex :type Integer))
  ;[1 1 1] Stop periodic damage when leaving
  (Utilities|Casting|CastToCapsuleComponent OtherComp)
  (Utilities|Time|ClearandInvalidateTimerbyHandle (Variables|Default|GetDamageTickTimer)))

(event Custom|DamageTick
  (Game|Damage|ApplyDamage (Variables|Default|GetChar) (Variables|Default|GetDamagePerTick) 0 0 "/Game/MyContent/Blueprints/BP_CausticDamageType.BP_CausticDamageType_C"))

(fn ConstructionScript
  (Components|Box|SetBoxExtent (Variables|Default|GetBox) (Math|Vector|MakeVector (Variables|Default|GetX) (Variables|Default|GetY) (Variables|Default|GetZ)) true))